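; Base weapon actor that handles timed firing, clip and reserve ammo, and delayed reloading, driven by the WeaponData struct.
; StartShooting fires immediately and starts a looping rate-of-fire timer, while StopShooting schedules an event for the remaining cooldown.
; MakeShot traces from the owner's camera or eyes, calls OnMakeShot, then spawns a muzzle projectile toward the aim point or applies hit-scan damage.
; Ammo counts and trace lines display as debug output.
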(event `self.ReceiveBeginPlay`
  (set `self.OwnerCamera` (`self.GetComponentByClass` (`self.GetOwner`) "/Script/Engine.CameraComponent"))
  (setmembers `/Game/Weapons/WeaponData/S_WeaponData` :`StructRef` (`self.WeaponData`) :`CurrentClipAmmo` (`self.GetCurrentClipAmmo`))
  (setmembers `/Game/Weapons/WeaponData/S_WeaponData` :`StructRef` (`self.WeaponData`) :`CurrentClipAmmo` (`self.GetCurrentWeaponAmmo`)))

(event `OnMakeShot`
  (params (Hit :type "HitResult Structure")))

(event `self.ReceiveTick`
  (params (DeltaSeconds :type "Float (single-precision)"))
  (`KismetSystemLibrary.PrintString` (`KismetTextLibrary.Conv_TextToString` (`|FormatText` "{WeaponName} - Ammo {Current} / {Max}" self (`self.GetCurrentClipAmmo`) (`self.GetCurrentWeaponAmmo`))) true true (struct :`G` 0.208333 :`B` 0.044066 :`A` 1.0) 0.0))

(fn `AddAmmo`
  (`|VariableSetRef` (`self.GetCurrentWeaponAmmo`) (`KismetMathLibrary.Min` (`.MaxWeaponAmmo_28_E6CBAEC44EE5B7B1EC8B988F6C374663` (break `/Game/Weapons/WeaponData/S_WeaponData` (`self.WeaponData`))) (+ (`self.GetCurrentWeaponAmmo`) (`self.GetCurrentClipAmmo`)))))

(fn `IsAmmoFull`
  (returns (Success :type Boolean))
  (return (== 0 (`self.GetMaxClipAmmo`))))

(fn `IsEnableForShooting`
  (set `self.IsReadyForShoot` true)
  (return))

(fn `MakeShot`
  (locals (L_OutHit :type "HitResult Structure") (L_Direction :type "Vector Structure" :default (0.0 0.0 0.0)))
  (bind ((`ProjectileClass_22_578AFE51450A2474C082DE9686AA9123` _projectileclass) (`Damage_24_DBA55E514F2C7CA125278F9B35CFBCFC` _damage)) (break `/Game/Weapons/WeaponData/S_WeaponData` (`self.WeaponData`)))
  (bind (_bblockinghit _binitialoverlap _time _distance _location _impactpoint _normal _impactnormal _physmat _hitactor _hitcomponent _hitbonename _bonename _hititem _elementindex _faceindex _tracestart _traceend) (`GameplayStatics.BreakHitResult` (`local.L_OutHit`)))
  (bind (_outlocation _outrotation) (`self.GetActorEyesViewPoint` (`self.GetOwner`)))
  (if (> (`self.GetCurrentClipAmmo`) 0)
    (`/Engine/EditorBlueprintResources/StandardMacros.IsValid` (`self.OwnerCamera`)
      (:`Is Valid`
        (bind _desiredview (`CameraComponent.GetCameraView` (`self.OwnerCamera`) 0.0))
        (bind (_location_2 _rotation) (break `MinimalViewInfo` _desiredview))
        (set `self.StartPoint` _location_2)
        (set `self.EndPoint` (+ (`self.StartPoint`) (* (`KismetMathLibrary.Conv_RotatorToVector` _rotation) (`self.TraceLengh`)))))
      (:`Is Not Valid`
        (set `self.StartPoint` _outlocation)
        (set `self.EndPoint` (+ (`self.StartPoint`) (* (`KismetMathLibrary.Conv_RotatorToVector` _outrotation) (`self.TraceLengh`))))))
    (bind (_outhit _returnvalue) (`KismetSystemLibrary.LineTraceSingle` (`self.StartPoint`) (`self.EndPoint`) "TraceTypeQuery2" false (`|MakeArray` (`self.GetOwner`)) "ForDuration" false (struct :`R` 1.0 :`A` 1.0) (struct :`G` 1.0 :`A` 1.0) 2.0))
    (set `local.L_OutHit` _outhit)
    (set `local.L_Direction` (`KismetMathLibrary.Normal` (- (`KismetMathLibrary.SelectVector` _impactpoint _traceend _returnvalue) (`SceneComponent.GetSocketLocation` (`self.WeaponMesh`) (`self.MuzzleFXSocketName`)))))
    (`self.OnMakeShot` (`local.L_OutHit`))
    (setmembers `/Game/Weapons/WeaponData/S_WeaponData` :`StructRef` (`self.WeaponData`) :`CurrentClipAmmo` (`KismetMathLibrary.Max` (- (`self.GetCurrentClipAmmo`) 1)))
    (switch `/Game/Weapons/WeaponData/ENUM_AmmoType` (`.AmmoType_23_EDCB648B450EF260F56D3E981F327C52` (break `/Game/Weapons/WeaponData/S_WeaponData` (`self.WeaponData`)))
      (:`NewEnumerator0`
        (`|SpawnActorFromClass` _projectileclass (`KismetMathLibrary.MakeTransform` (`SceneComponent.GetSocketLocation` (`self.WeaponMesh`) (`self.MuzzleFXSocketName`))) "AdjustIfPossibleButAlwaysSpawn" "MultiplyWithRoot" (`self.GetOwner`) _damage (`local.L_Direction`) null)
        (`KismetSystemLibrary.PrintString` (`KismetSystemLibrary.GetClassDisplayName` _projectileclass) true true (struct :`G` 0.66 :`B` 1.0 :`A` 1.0) 5.0)
        (return))
      (:`NewEnumerator1`
        (`GameplayStatics.ApplyDamage` (`.HitActor` (`GameplayStatics.BreakHitResult` (`local.L_OutHit`))) (`KismetMathLibrary.Conv_IntToDouble` (`.Damage_24_DBA55E514F2C7CA125278F9B35CFBCFC` (break `/Game/Weapons/WeaponData/S_WeaponData` (`self.WeaponData`)))) (`self.OwnerController`) self)
        (return)))))

(fn `Reload`
  (locals (L_AmmoNeeded :type Integer))
  (set `local.L_AmmoNeeded` (- (`self.GetMaxClipAmmo`) (`self.GetCurrentClipAmmo`)))
  (if (>= (`self.GetCurrentWeaponAmmo`) (`local.L_AmmoNeeded`))
    (setmembers `/Game/Weapons/WeaponData/S_WeaponData` :`StructRef` (`self.WeaponData`) :`CurrentClipAmmo` (+ (`local.L_AmmoNeeded`) (`self.GetCurrentClipAmmo`)))
    (setmembers `/Game/Weapons/WeaponData/S_WeaponData` :`StructRef` (`self.WeaponData`) :`CurrentWeaponAmmo` (- (`self.GetCurrentWeaponAmmo`) (`local.L_AmmoNeeded`)))
    (`self.OnReloadFinished`)
    (return)
    (else
      (setmembers `/Game/Weapons/WeaponData/S_WeaponData` :`StructRef` (`self.WeaponData`) :`CurrentClipAmmo` (+ (`self.GetCurrentClipAmmo`) (`self.GetCurrentWeaponAmmo`)))
      (setmembers `/Game/Weapons/WeaponData/S_WeaponData` :`StructRef` (`self.WeaponData`) :`CurrentWeaponAmmo` 0)
      (`self.OnReloadFinished`)
      (return))))

(fn `Start Reloading`
  (returns (Success :type Boolean))
  (`KismetSystemLibrary.K2_SetTimerDelegate` (`|CreateDelegate` :!event `Reload`) (`.ReloadTime_30_820580B4405F684A8A1D46920217D0AF` (break `/Game/Weapons/WeaponData/S_WeaponData` (`self.WeaponData`))))
  (return true))

(fn `StartShooting`
  (returns (Success :type Boolean))
  (if (`self.IsReadyForShoot`)
    (bind _aspawn (cast `Pawn` (`self.GetOwner`)))
    (set `self.OwnerController` (`Pawn.GetController` _aspawn))
    (`self.MakeShot`)
    (`self.StartShootTimer` (`|CreateDelegate` :!event `MakeShot`))
    (set `self.IsReadyForShoot` false)
    (return true)
    (else
      (return false))))

(fn `StartShootTimer`
  (params (Event :type Delegate))
  (bind _returnvalue (`KismetSystemLibrary.K2_SetTimerDelegate` Event (`.RateOfFire_29_CDF8D72849F4B3F20D2940ADB916A9D2` (break `/Game/Weapons/WeaponData/S_WeaponData` (`self.WeaponData`))) true))
  (set `self.ShootTimer` _returnvalue))

(fn `StopShooting`
  (returns (Success :type Boolean))
  (if (`KismetSystemLibrary.K2_IsTimerActiveHandle` (`self.ShootTimer`))
    (`KismetSystemLibrary.K2_SetTimerDelegate` (`|CreateDelegate` :!event `IsEnableForShooting`) (`KismetSystemLibrary.K2_GetTimerRemainingTimeHandle` (`self.ShootTimer`)))
    (`KismetSystemLibrary.K2_ClearAndInvalidateTimerHandle` (`self.ShootTimer`))
    (return true)
    (else
      (return false))))

(fn `UserConstructionScript`)