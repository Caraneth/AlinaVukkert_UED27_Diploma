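; Base enemy Blueprint that handles damage, attacking, death and target-death checks.
; Damage reduces BPACHealth, then either alerts BP_EnemyAIController or calls StartDeath, which flags IsDead and starts BPACAttackAction.
; AttackPlayer triggers that same action component, while CheckIsTargetDead clears the blackboard's CanSeePlayer key and IsAttacking when the player's health runs out.
; Tick draws the AI manager's patrol state above the capsule as debug text.
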(event `self.ReceiveBeginPlay`
  (add `self.OnTakeAnyDamage` (`|CreateDelegate` :!event `ApplyDamage`)))

(event `self.ReceiveTick`
  (params (DeltaSeconds :type "Float (single-precision)"))
  (`KismetSystemLibrary.DrawDebugString` (+ (`SceneComponent.K2_GetComponentLocation` (`self.CapsuleComponent`)) (0.0 0.0 20.0)) (`KismetTextLibrary.Conv_TextToString` (`|FormatText` "{CurrentPatrolState} " (`|GetEnumeratorNameAsString` (`/Game/Components/BPAC_AIPatrollingManager.PatrolState` (`self.BPAC_AIManager`))))) null (struct :`G` 0.14996 :`B` 0.122139 :`A` 1.0)))

(fn `ApplyDamage`
  (params (DamagedActor :type "Actor Object Reference") (Damage :type "Float (single-precision)") (DamageType :type "DamageType Object Reference") (InstigatedBy :type "Controller Object Reference") (DamageCauser :type "Actor Object Reference"))
  (`/Game/Components/BPAC_EntityResourceBase.DecreaseValue` (`self.BPAC_Health`) (`KismetMathLibrary.FTrunc` Damage))
  (if (> (`/Game/Components/BPAC_EntityResourceBase.GetCurrentValue` (`self.BPAC_Health`)) 0)
    (bind _asbp_enemy_aicontroller (cast `/Game/Enemy/AI/BP_EnemyAIController` (`AIBlueprintHelperLibrary.GetAIController` self)))
    (`/Game/Enemy/AI/BP_EnemyAIController.AttackedbyPlayer` _asbp_enemy_aicontroller)
    (else
      (`self.StartDeath`))))

(fn `AttackPlayer`
  (params (AttackingActor :type "Actor Object Reference"))
  (`/Game/Components/BPAC_ActionBase.StartAction` (`self.BPAC_AttackAction`) AttackingActor))

(fn `CheckIsTargetDead`
  (returns (Dead :type Boolean))
  (if (<= (`/Game/Components/BPAC_EntityResourceBase.GetCurrentValue` (`self.GetComponentByClass` (`GameplayStatics.GetPlayerCharacter` 0) "/Game/Components/BPAC_Health.BPAC_Health_C")) 0)
    (`BlackboardComponent.SetValueAsBool` (`AIBlueprintHelperLibrary.GetBlackboard` null) "CanSeePlayer" false)
    (set `self.IsAttacking` false)
    (return true)
    (else
      (return false))))

(fn `StartDeath`
  (if (not (`self.IsDead`))
    (`/Game/Components/BPAC_ActionBase.StartAction` (`self.BPAC_AttackAction`) null)
    (set `self.IsDead` true)))

(fn `UserConstructionScript`)