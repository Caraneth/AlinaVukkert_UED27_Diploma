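; Enemy AI controller that runs BT_EnemyAI and turns perception events into chase, search and patrol behavior.
; Sensing a tagged actor or calling AttackedbyPlayer sets the blackboard target and switches BPACAIState to chasing.
; Losing sight switches to looking for the player and starts a memory timer that clears the target and resumes patrolling.
; Player perception updates also store LastTargetPoint; Tick prints AIState for debugging.
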(event `self.ReceiveBeginPlay`
  (`self.RunBehaviorTree` "/Game/Enemy/AI/BT_EnemyAI.BT_EnemyAI"))

(event `self.AIPerception.OnTargetPerceptionUpdated`
  (params (Actor :type "Actor Object Reference") (Stimulus :type "AIStimulus Structure"))
  (set `self.TargetActor` Actor)
  (if (>= (`KismetArrayLibrary.Array_Find` (`Actor.Tags` (`self.TargetActor`)) (`self.EnemyTag`)) 0)
    (if (`.bSuccessfullySensed` (break `AIStimulus` Stimulus))
      (`self.FollowNewActorTarget` (`self.TargetActor`))
      (`BlackboardComponent.SetValueAsBool` (`AIBlueprintHelperLibrary.GetBlackboard` null) "CanSeePlayer" true)
      (else
        (`BlackboardComponent.SetValueAsBool` (`AIBlueprintHelperLibrary.GetBlackboard` null) "CanSeePlayer" false)
        (`self.LookingForPlayer`)))))

(event `self.AIPerception.OnPerceptionUpdated`
  (params (UpdatedActors :type "Array of Actor Object Reference (by ref)"))
  (if (`KismetArrayLibrary.Array_Contains` UpdatedActors (`GameplayStatics.GetPlayerCharacter` 0))
    (`BlackboardComponent.SetValueAsObject` (`AIBlueprintHelperLibrary.GetBlackboard` null) (`self.ChasingTargetKey`) (`GameplayStatics.GetPlayerCharacter` 0))
    (`BlackboardComponent.SetValueAsVector` (`AIBlueprintHelperLibrary.GetBlackboard` null) "LastTargetPoint" (`self.K2_GetActorLocation` (`GameplayStatics.GetPlayerCharacter` 0)))))

(event `self.ReceiveTick`
  (params (DeltaSeconds :type "Float (single-precision)"))
  (`KismetSystemLibrary.PrintString` (`KismetStringLibrary.Conv_ByteToString` (`BlackboardComponent.GetValueAsEnum` (`AIBlueprintHelperLibrary.GetBlackboard` null) "AIState")) true true (struct :`G` 0.66 :`B` 1.0 :`A` 1.0) 0.0))

(fn `AttackedbyPlayer`
  (`self.FollowNewActorTarget` (`GameplayStatics.GetPlayerCharacter` 0))
  (`BlackboardComponent.SetValueAsBool` (`AIBlueprintHelperLibrary.GetBlackboard` null) "CanSeePlayer" true))

(fn `ClearAIMemory`
  (`BlackboardComponent.SetValueAsObject` (`AIBlueprintHelperLibrary.GetBlackboard` null) (`self.ChasingTargetKey`) null)
  (`/Game/Components/BPAC_AIStateMachine.SetPatrollingState` (`self.BPAC_AIState`))
  (return))

(fn `FollowNewActorTarget`
  (params (FollowTargetActor :type "Actor Object Reference"))
  (`KismetSystemLibrary.K2_ClearAndInvalidateTimerHandle` (`self.MemoryTimer`))
  (`BlackboardComponent.SetValueAsObject` (`AIBlueprintHelperLibrary.GetBlackboard` null) (`self.ChasingTargetKey`) FollowTargetActor)
  (`/Game/Components/BPAC_AIStateMachine.SetChasingState` (`self.BPAC_AIState`))
  (return))

(fn `LookingForPlayer`
  (`/Game/Components/BPAC_AIStateMachine.SetLookingForPlayerState` (`self.BPAC_AIState`))
  (bind _returnvalue (`KismetSystemLibrary.K2_SetTimer` null "ClearAIMemory" (`self.MemoryDuration`)))
  (set `self.MemoryTimer` _returnvalue)
  (return))

(fn `UserConstructionScript`)